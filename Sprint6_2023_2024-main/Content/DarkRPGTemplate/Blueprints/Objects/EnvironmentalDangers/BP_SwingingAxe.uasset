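; BP_SwingingAxe is an environmental hazard, an axe that swings back and forth and damages actors it touches.
; A looping timeline started on BeginPlay scales MaxSwing by a multiplier between -1 and 1 to drive the axe's roll.
; A box overlap applies heavy environmental damage to the overlapping actor.
; Tick uses a Delay to play a swipe sound every two seconds, timed independently of the swing timeline.
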(event OnComponentBeginOverlap(Box)
  (params (OverlappedComponent :type Primitive%20Component%20Object%20Reference) (OtherActor :type Actor%20Object%20Reference) (OtherComp :type Primitive%20Component%20Object%20Reference) (OtherBodyIndex :type Integer) (bFromSweep :type Boolean) (SweepResult :type Hit%20Result%20Structure%20%28by%20ref%29))
  (Game|Damage|ApplyDamage OtherActor 1e+02 0 0 "/Engine/EngineDamageTypes/DmgTypeBP_Environmental.DmgTypeBP_Environmental_C") ; When the box collision overlaps, deal damage\nto the overlapping actor
)

(event EventBeginPlay
  (bind _mult (Timeline|AxeSwingTimeline Play) ; Timeline automatically loops\nBegins at -1, goes to 1 and then\nback to -1
    (:Update
      (Transformation|SetRelativeRotation (Variables|Default|GetAxe) (Math|Rotator|MakeRotator (* _mult (Variables|Default|GetMaxSwing)) 0.0 0.0) false false) ; Update axe rotation
    )))

(event EventTick
  (params (DeltaSeconds :type Float%20%28single-precision%29))
  (Utilities|FlowControl|Delay 2.0)
  (Audio|PlaySoundatLocation "/Game/DarkRPGTemplate/Audio/Cues/SC_SwipeCue.SC_SwipeCue" (Transformation|GetActorLocation) "0, 0, 0" 0.8 0.2 0.0 "/Game/DarkRPGTemplate/Audio/DefaultSoundAttenutation.DefaultSoundAttenutation" 0 0 0) ; Play swinging noise every 2 seconds
)

(fn ConstructionScript)