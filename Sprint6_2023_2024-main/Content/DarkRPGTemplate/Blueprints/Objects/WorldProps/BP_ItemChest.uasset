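; BP_ItemChest is a one-time-use chest prop that gives the player a random item.
; Use destroys the use trigger, plays player and chest open animations, and opens a Tick gate that interpolates the user to the use point.
; After the montage-length delay, it closes the gate and spawns a pickup from PossibleItems at ItemPoint.
; The pickup's trigger moves to the use point, keeping it outside the chest mesh.
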(event Custom|OpenGate
  (bind _usepoint (Variables|Default|GetUsepoint))
  (bind _returnvalue (Transformation|GetWorldLocation _usepoint))
  (bind (_x _y) (Math|Vector|BreakVector _returnvalue))
  (Utilities|FlowControl|Gate true) ; enters at Open
)

(event Custom|CloseGate
  (bind _usepoint (Variables|Default|GetUsepoint))
  (bind _returnvalue (Transformation|GetWorldLocation _usepoint))
  (bind (_x _y) (Math|Vector|BreakVector _returnvalue))
  (Utilities|FlowControl|Gate true) ; enters at Close
)

(event EventUse
  (params (User :type Pawn%20Object%20Reference))
  (bind _possibleitems (Variables|Default|GetPossibleItems))
  (Components|DestroyComponent (Variables|Default|GetUseTrigger)) ; Destroy the use component of the chest so it can't be used again
  (bind _output_get (Variables|Default|SetUser User))
  (bind _asbp_player (Utilities|Casting|CastToBP_Player _output_get))
  ;[1 1 1] Play animations when used
  (bind _montagelength (Default|PlayMontage _asbp_player "/Game/DarkRPGTemplate/Animations/Player/Anim_BaseMale_ChestOpen_Montage.Anim_BaseMale_ChestOpen_Montage"))
  (Audio|Components|Audio|Play (Variables|Default|GetChest) false)
  (CallFunction|OpenGate) ; Begin the location interpolation
  (Utilities|FlowControl|Delay _montagelength) ; After anim has finished
  (CallFunction|CloseGate) ; Stop location interp
  (bind _returnvalue (Game|SpawnActorfromClass "/Game/DarkRPGTemplate/Blueprints/Objects/BP_PickupObject.BP_PickupObject_C" (Transformation|GetWorldTransform (Variables|Default|GetItemPoint)) "Undefined" "OverrideRootScale" 0 (Utilities|Array|Get(acopy) _possibleitems (Math|Random|RandomInteger (Utilities|Array|Length _possibleitems))) 0)) ; Create a pickup object with a random possible item
  (Transformation|SetWorldLocation (Variables|/Game/DarkRPGTemplate/Blueprints/Objects/BP_UsableObject.BP_UsableObject_C|GetUseTrigger _returnvalue) (Transformation|GetWorldLocation (Variables|Default|GetUsepoint)) false false) ; Move its use trigger to the player so it's not inside the chest mesh
)

(event EventTick
  (params (DeltaSeconds :type Float%20%28single-precision%29))
  (bind _usepoint (Variables|Default|GetUsepoint))
  (bind _returnvalue (Transformation|GetWorldLocation _usepoint))
  (bind (_x _y) (Math|Vector|BreakVector _returnvalue))
  (Utilities|FlowControl|Gate true
    (:Exit
      (CallFunction|InterpActortoLocationandRotation (Variables|Default|GetUser) (Math|Vector|MakeVector _x _y (.Z (Math|Vector|BreakVector (Transformation|GetActorLocation (Variables|Default|GetUser))))) (Transformation|GetWorldRotation (Variables|Default|GetUsepoint)) 8.0 true true) ; Interp the user to the correct location for the animation
    )))

(fn ConstructionScript
  (|CallParentFunction))