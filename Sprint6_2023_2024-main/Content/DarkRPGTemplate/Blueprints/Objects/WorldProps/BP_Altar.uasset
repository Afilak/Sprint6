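; BP_Altar is an interactable prayer altar that registers itself as the user's last used altar.
; Each use alternates via a FlipFlop between starting and stopping prayer through messages to player pawn 0, locking movement while praying.
; A Tick gate turns the player toward the altar's bowl until the end-pray animation delay finishes, then movement is restored.
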(event Custom|OpenGate
  (bind _player (Variables|Default|GetPlayer))
  (bind _bowl (Variables|Default|GetBowl))
  (bind _returnvalue (Transformation|GetActorLocation _player))
  (bind _returnvalue_2 (Transformation|GetWorldLocation _bowl))
  (bind (_x _y) (Math|Vector|BreakVector _returnvalue_2))
  (Utilities|FlowControl|Gate true) ; enters at Open
)

(event Custom|CloseGate
  (bind _player (Variables|Default|GetPlayer))
  (bind _bowl (Variables|Default|GetBowl))
  (bind _returnvalue (Transformation|GetActorLocation _player))
  (bind _returnvalue_2 (Transformation|GetWorldLocation _bowl))
  (bind (_x _y) (Math|Vector|BreakVector _returnvalue_2))
  (Utilities|FlowControl|Gate true) ; enters at Close
)

(event EventUse
  (params (User :type Pawn%20Object%20Reference))
  (bind _player (Variables|Default|GetPlayer))
  (Class|BPPawnInteractionInterface|SetLastAltar(Message) User self) ; Updates the player's last used altar to\nthis altar
  (Utilities|FlowControl|FlipFlop
    (:A
      (CallFunction|OpenGate) ; Begins forced rotation of player
      (Class|BPPawnInteractionInterface|Begin/EndPray(Message) (Variables|Default|GetPlayer) true) ; Tells the player to start praying
      (Class|BPPawnInteractionInterface|ActorCanMove(Message) _player false) ; Disables player movement while praying
    )
    (:B
      (bind _duration (Class|BPPawnInteractionInterface|Begin/EndPray(Message) (Variables|Default|GetPlayer) false)) ; Tells the player to stop praying
      (Utilities|FlowControl|Delay _duration) ; Waits until player has finished \nreturning from pray animation
      (CallFunction|CloseGate) ; Stops rotation of player
      (Class|BPPawnInteractionInterface|ActorCanMove(Message) _player true) ; Allows the player to move again
    )))

(event EventBeginPlay
  (Variables|Default|SetPlayer (Game|Player|GetPlayerPawn 0)))

(event EventTick
  (params (DeltaSeconds :type Float%20%28single-precision%29))
  (bind _player (Variables|Default|GetPlayer))
  (bind _bowl (Variables|Default|GetBowl))
  (bind _returnvalue (Transformation|GetActorLocation _player))
  (bind _returnvalue_2 (Transformation|GetWorldLocation _bowl))
  (bind (_x _y) (Math|Vector|BreakVector _returnvalue_2))
  (Utilities|FlowControl|Gate true
    (:Exit
      (CallFunction|InterpActortoLocationandRotation (Variables|Default|GetPlayer) "0, 0, 0" (Math|Rotator|FindLookatRotation _returnvalue (Math|Vector|MakeVector _x _y (.Z (Math|Vector|BreakVector _returnvalue)))) 8.0 true false) ; Forces the player to face the altar
    )))

(fn ConstructionScript
  (|CallParentFunction))