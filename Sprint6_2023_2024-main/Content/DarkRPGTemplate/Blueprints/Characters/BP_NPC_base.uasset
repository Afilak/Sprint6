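; Base NPC character for the Dark RPG template, handling AI-triggered montage attacks, damage, stagger and death.
; It turns smoothly toward its AI focus and yaws a health bar, shown once damaged, toward the camera.
; Damage notifies listeners such as the vision service and plays hit reactions; death awards XP and may drop a random item.
; Physical animation simulates lower bones, blending death montages into full ragdoll, while environmental kills ragdoll immediately.
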(event Custom|AttackEvent
  ;[1 1 1] Called by AI
  (Utilities|Attack))

(event EventBeginPlay
  ;[1 1 1] Physical animation initialisation
  (Class|PhysicalAnimationComponent|SetSkeletalMeshComponent (Variables|Default|GetPhysicalAnimation) (Variables|Character|GetMesh)) ; Assigns character mesh as the target\nof physical animation component
  (Class|PhysicalAnimationComponent|ApplyPhysicalAnimationProfileBelow (Variables|Default|GetPhysicalAnimation) (Variables|Misc|GetSimulateBoneName) "DefaultProfile" false false) ; Applies profile set in phat to bones below\n"simulate bone name"
  (Class|SkeletalMeshComponent|SetAllBodiesBelowSimulatePhysics (Variables|Character|GetMesh) (Variables|Misc|GetSimulateBoneName) true false) ; Sets bones below "simulate bone name"\nto simulate physics
)

(event Game|Damage|EventAnyDamage
  (params (Damage :type Float%20%28single-precision%29) (DamageType :type Damage%20Type%20Object%20Reference) (InstigatedBy :type Controller%20Object%20Reference) (DamageCauser :type Actor%20Object%20Reference))
  ;[1 1 1] Handles damage
  (Utilities|TakeDamage Damage DamageCauser DamageType))

(event EventStagger
  ;[1 1 1] Stagger handling
  (CallFunction|ActorCanMove false) ; Prevent movement\nwhile staggered
  (bind _montagelength (CallFunction|PlayMontage (Variables|Animations|GetStaggerAnimation)))
  (Utilities|FlowControl|Delay _montagelength) ; After montage is complete
  (CallFunction|ActorCanMove true) ; Re-enable movement
)

(event EventTick
  (params (DeltaSeconds :type Float%20%28single-precision%29))
  (bind _self self)
  (bind _healthbar (Variables|Default|GetHealthBar))
  (bind _returnvalue (AI|GetAIController _self))
  (bind _returnvalue_2 (Transformation|GetWorldRotation _healthbar))
  (bind _returnvalue_3 (Class|AIController|GetFocusActor _returnvalue))
  (bind (_roll _pitch) (Math|Rotator|BreakRotator _returnvalue_2))
  ;[1 1 1] Tick
  (Transformation|SetWorldRotation (Variables|Default|GetHealthBar) (Math|Rotator|MakeRotator _roll _pitch (.Yaw (Math|Rotator|BreakRotator (Math|Rotator|FindLookatRotation (Transformation|GetActorLocation) (Transformation|GetActorLocation (Game|GetPlayerCameraManager 0)))))) false false) ; Update health bar rotation every tick
  (Utilities|IsValid _returnvalue ; Avoid accessed none errors\nEnsure AI controller exists
    (:Is%20Valid
      (Utilities|IsValid _returnvalue_3
        (:Is%20Valid
          (CallFunction|RotateTowardsFocus _returnvalue_3) ; Update NPC rotation to face target
        )))))

(event EventActorCanMove
  (params (CanMove :type Boolean))
  ;[1 1 1] Enables/Disables movement
  (Variables|/Script/Engine.CharacterMovementComponent|SetMaxWalkSpeed (Variables|Character|GetCharacterMovement) (select CanMove 2.5e+02 0.0)))

(fn ConstructionScript
  (Variables|Misc|SetInitialTransform (Transformation|GetActorTransform)) ; Sets initial transform where the NPC is placed, for used when being respawned
)

(fn PlayMontage
  (params (Montage :type Anim%20Montage%20Object%20Reference))
  (bind _returnvalue (Animation|Montage|MontagePlay (Components|SkeletalMesh|GetAnimInstance (Variables|Character|GetMesh)) Montage 1.0 "MontageLength" 0.0 true))
  (return _returnvalue))

(fn DropItems
  (bind _returnvalue (Transformation|GetActorLocation))
  (bind _itemstodrop (Variables|Items|GetItemsToDrop))
  (bind (_x _y _z) (Math|Vector|BreakVector _returnvalue))
  (Game|SpawnActorfromClass "/Game/DarkRPGTemplate/Blueprints/Objects/BP_PickupObject.BP_PickupObject_C" (Math|Transform|MakeTransform (Math|Vector|MakeVector _x _y (- _z (Variables|/Script/Engine.CapsuleComponent|GetCapsuleHalfHeight (Variables|Collision|GetCapsuleComponent))))) "AlwaysSpawn" "OverrideRootScale" 0 (Utilities|Array|Get(acopy) _itemstodrop (Math|Random|RandomInteger (Utilities|Array|Length _itemstodrop))) 0) ; Spawn an instance of "PickupObject" and input the inventory\nitem class as a parameter
)

(fn EnableHealthBar
  (params (Enable :type Boolean))
  (Rendering|SetVisibility (Variables|Default|GetHealthBar) Enable false))

(fn UpdateHealthBar
  (bind _health (Variables|Stats|GetHealth))
  (bind _maxhealth (Variables|Stats|GetMaxHealth))
  (Class|BPUIInterface|UpdateHealth(Message) (UserInterface|GetUserWidgetObject (Variables|Default|GetHealthBar)) _health _maxhealth)
  (Development|PrintString (Utilities|String|Append "Health: " (Utilities|String|ToString(Float) _health) "Max Health: " (Utilities|String|ToString(Float) _maxhealth))))

(fn RotateTowardsFocus
  (params (FocusedActor :type Actor%20Object%20Reference))
  (bind _returnvalue (Transformation|GetActorRotation))
  (bind (_roll _pitch) (Math|Rotator|BreakRotator _returnvalue))
  (bind _output_get (LocalVariables|SetLocalFocusedActor FocusedActor))
  (if (not (Math|Rotator|Equal(Rotator) (Transformation|GetActorRotation) (Math|Rotator|MakeRotator _roll _pitch (.Yaw (Math|Rotator|BreakRotator (Math|Rotator|FindLookatRotation (Transformation|GetActorLocation) (Transformation|GetActorLocation _output_get))))) 0.0001)) ; If already facing towards target,\ndon't bother updating
    (LocalVariables|SetLookAtRotation (Math|Rotator|MakeRotator _roll _pitch (.Yaw (Math|Rotator|BreakRotator (Math|Rotator|FindLookatRotation (Transformation|GetActorLocation) (Transformation|GetActorLocation _output_get))))))
    (Transformation|SetActorRotation (Math|Interpolation|RInterpTo (Transformation|GetActorRotation) (LocalVariables|GetLookAtRotation) (Utilities|Time|GetWorldDeltaSeconds) (Variables|Stats|GetTurnSpeed))) ; Update rotation with Rinterp output
  ))

(fn ActorCanBleed
  (return (Variables|Misc|GetBleeds)))

(fn AddtoUserInventory
  (params (InventoryItem :type BP%20Inventory%20Item%20Class%20Reference))
  (return false))

(fn Begin/EndPray
  (params (Begin :type Boolean))
  (return 0.0))

(fn GetFaction
  (return (Variables|Stats|GetFaction)))

(fn GetIsDead
  (return (<= (Variables|Stats|GetHealth) 0.0)))

(fn GetTorsoMontage
  (return false))

(fn GetWeapon
  (bind _asbp_weapon (Utilities|Casting|CastToBP_Weapon (Variables|/Script/Engine.ChildActorComponent|GetChildActor (Variables|Default|GetWeapon)))
    (:then
      _)
    (:CastFailed
      _))
  (return _asbp_weapon))

(fn GetXPWorth
  (return (Variables|Stats|GetXPWorth)))